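; Base 2D side-scroller player character with horizontal movement, jumping, health and a health bar widget.
; Each tick it derives an Idle, Run, Jump or Fall state from velocity to pick the flipbook, and flips control yaw to face the travel direction.
; Damage clamps health, refreshes the widget and triggers a one-time death that only prints a message.
; The H key applies self-damage for testing.
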(event `self.ReceiveBeginPlay`
  (set `self.MovementState` "NewEnumerator4")
  (bind _returnvalue (`|CreateWidget` "/Game/Blueprints/UI/WBP_PlayerHealth.WBP_PlayerHealth_C"))
  (bind _output_get (set `self.HealthWidgetRef` _returnvalue))
  (`UserWidget.AddToViewport` _output_get 0)
  (`self.UpdateHealth`))

(event `self.ReceiveTick`
  (params (DeltaSeconds :type "Float (single-precision)"))
  (`|ExecutionSequence`
    (:`then_0`
      (`self.UpdateFlipBook`))
    (:`then_1`
      (`self.UpdatePlayerRotation`))))

(event `Key|H`
  (params (Key :type "Key Structure"))
  ;[1 1 1] Damage tester
  (:`Pressed`
    (`GameplayStatics.ApplyDamage` self 20.0)))

(event `self.ReceiveAnyDamage`
  (params (Damage :type "Float (single-precision)") (DamageType :type "DamageType Object Reference") (InstigatedBy :type "Controller Object Reference") (DamageCauser :type "Actor Object Reference"))
  (set `self.Health` (`KismetMathLibrary.FClamp` (- (`self.Health`) Damage) 0.0 (`self.DefualtHealth`)))
  (`self.UpdateHealth`)
  (if (and (<= (`self.Health`) 0.0) (not (`self.IsDead`)))
    (set `self.IsDead` true)
    (`self.PlayerDied`)))

(event `InputAxis|MoveRight`
  (params (AxisValue :type "Float (single-precision)"))
  ;[1 1 1] Handles Jump
  (`self.AddMovementInput` (1.0 0.0 0.0) AxisValue))

(event `InputAction|Jump`
  (params (Key :type "Key Structure"))
  ;[1 1 1] Handles Holding Jump
  (:`Pressed`
    (`self.Jump`))
  (:`Released`
    (`self.StopJumping`)))

(fn `PlayerDied`
  (`KismetSystemLibrary.PrintString` "You're Dead"))

(fn `UpdateFlipBook`
  (bind (_returnvalue_x _returnvalue_y _returnvalue_z) (`KismetMathLibrary.BreakVector` (`self.GetVelocity`)))
  (set `self.MovementState` (select `bool` (!= (`KismetMathLibrary.VSize` (`self.GetVelocity`)) 0.0) :`false` "NewEnumerator0" :`true` (select `bool` (`NavMovementComponent.IsFalling` (`self.CharacterMovement`)) :`false` "NewEnumerator1" :`true` (select `bool` (<= _returnvalue_z 0.0) :`false` "NewEnumerator2" :`true` "NewEnumerator3" :!type "/Game/Blueprints/EPlayerMovement Enum"))))
  (`PaperFlipbookComponent.SetFlipbook` (`self.Sprite`) (select `/Game/Blueprints/EPlayerMovement` (`self.MovementState`) :`NewEnumerator0` (`self.FB_Idel`) :`NewEnumerator1` (`self.FB_Run`) :`NewEnumerator2` (`self.FB_Jump`) :`NewEnumerator3` (`self.FB_Fall`))))

(fn `UpdateHealth`
  (`/Game/Blueprints/UI/WBP_PlayerHealth.UpdateHealth` (`self.HealthWidgetRef`) (`self.Health`) (`self.DefualtHealth`)))

(fn `UpdatePlayerRotation`
  (bind _returnvalue_x (`KismetMathLibrary.BreakVector` (`self.GetVelocity`)))
  (`/Engine/EditorBlueprintResources/StandardMacros.CompareFloat` _returnvalue_x
    (:`>`
      (`Controller.SetControlRotation` (`GameplayStatics.GetPlayerController` 0) (`KismetMathLibrary.MakeRotator` 0.0)))
    (:`<`
      (`Controller.SetControlRotation` (`GameplayStatics.GetPlayerController` 0) (`KismetMathLibrary.MakeRotator` 0.0 0.0 180.0)))))

(fn `UserConstructionScript`
  (set `self.Health` (`self.DefualtHealth`)))