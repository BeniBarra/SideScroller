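; Bat enemy that moves back and forth along the world X axis, starting in a random direction.
; Tick feeds constant movement input, and capsule hits with a nonzero X normal reverse MoveRight unless the player is hit.
; ToggleFacingDirection negates the sprite's current X scale only when MoveRight is true, so turning left leaves it unchanged.
; EnemyDied runs the parent logic, then destroys the actor.
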(event `self.ReceiveBeginPlay`
  (set `self.Move Right` (`KismetMathLibrary.RandomBool`))
  (`self.ToggleFacingDirection`))

(event `self.ReceiveTick`
  (params (DeltaSeconds :type "Float (single-precision)"))
  (`self.AddMovementInput` (1.0 0.0 0.0) (select `bool` (`self.Move Right`) :`false` -1.0 :`true` 1.0 :!type "Float (single-precision)")))

(event `self.CapsuleComponent.OnComponentHit`
  (params (HitComponent :type "PrimitiveComponent Object Reference") (OtherActor :type "Actor Object Reference") (OtherComp :type "PrimitiveComponent Object Reference") (NormalImpulse :type "Vector Structure") (Hit :type "HitResult Structure (by ref)"))
  ;[1 1 1] Don't change direction if collision target is player
  (if (!= OtherActor (`GameplayStatics.GetPlayerPawn` 0))
    (if (!= (.x Hit_Normal) 0.0)
      (set `self.Move Right` (not (`self.Move Right`)))
      (`self.ToggleFacingDirection`))))

(fn `EnemyDied`
  (`parent.EnemyDied`)
  (`self.K2_DestroyActor`))

(fn `ToggleFacingDirection`
  (bind (_returnvalue_x _returnvalue_y _returnvalue_z) (`KismetMathLibrary.BreakVector` (`SceneComponent.K2_GetComponentScale` (`self.Sprite`))))
  (`SceneComponent.SetWorldScale3D` (`self.Sprite`) (`KismetMathLibrary.MakeVector` (* _returnvalue_x (select `bool` (`self.Move Right`) :`false` 1.0 :`true` -1.0 :!type "Float (single-precision)")) _returnvalue_y _returnvalue_z)))

(fn `UserConstructionScript`
  (`parent.UserConstructionScript`))